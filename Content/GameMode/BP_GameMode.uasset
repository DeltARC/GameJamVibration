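; BP_GameMode is the game mode that tracks countdown time, score and remaining cartons, and shows them on a WB_Timer widget.
; BeginPlay starts a looping one-second timer and creates the widget, whose TimeLeft each tick updates with no end check.
; UpdateScore adds PointsLoseOrWin to the widget-held score, then stores that sum plus the points again as FinalScore.
; CartonLeft decrements the carton count and pushes it to the widget.
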(event Custom|UpdateTimer
  (bind _result (Math|Integer|DecrementInt (Variables|Default|GetTimerUpdater))
    (:%20%20
      (Variables|/Game/Widget/WB_Timer.WB_Timer_C|SetTimeLeft (Variables|Default|GetTimerRef) _result))))

(event Custom|UpdateScore
  (bind _timerref (Variables|Default|GetTimerRef))
  (Variables|/Game/Widget/WB_Timer.WB_Timer_C|SetScore _timerref (+ (Variables|/Game/Widget/WB_Timer.WB_Timer_C|GetScore _timerref) (Variables|Default|GetPointsLoseOrWin)))
  (Variables|Default|SetFinalScore (+ (Variables|/Game/Widget/WB_Timer.WB_Timer_C|GetScore _timerref) (Variables|Default|GetPointsLoseOrWin))))

(event Custom|CartonLeft
  (bind _result (Math|Integer|DecrementInt (Variables|Default|GetNumberOfCarton))
    (:%20%20
      (Variables|/Game/Widget/WB_Timer.WB_Timer_C|SetCartons (Variables|Default|GetTimerRef) _result))))

(event EventBeginPlay
  (Utilities|Time|SetTimerbyEvent (delegate Custom|UpdateTimer) 1.0 true)
  (bind _returnvalue (UserInterface|CreateWidget "/Game/Widget/WB_Timer.WB_Timer_C"))
  (bind _output_get (Variables|Default|SetTimerRef _returnvalue))
  (UserInterface|Viewport|AddtoViewport _output_get 0))

(fn ConstructionScript)