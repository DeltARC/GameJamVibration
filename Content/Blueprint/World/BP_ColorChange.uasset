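; World actor that tints a referenced directional light toward red as the game mode's timer runs down.
; On BeginPlay it caches the game mode and player character, then starts a fast looping timer, apparently to drive ChangeColor instead of Tick.
; While time remains, ChangeColor scales green and blue from TimeLeft within clamped limits, keeping red and alpha unchanged.
; The cached character's camera post-process nodes are unused.
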(event Custom|ChangeColor
  (bind _as_bp_game_mode (Variables|Default|GetAs%20BP%20Game%20Mode))
  (bind _directionnallight (Variables|Default|GetDirectionnalLight))
  (bind _timerref (Variables|/Game/GameMode/BP_GameMode.BP_GameMode_C|GetTimerRef _as_bp_game_mode))
  (bind _lightcomponent (Variables|/Script/Engine.Light|GetLightComponent _directionnallight))
  (bind _returnvalue (Rendering|Components|Light|GetLightColor _lightcomponent))
  (bind _timeleft (Variables|/Game/Widget/WB_Timer.WB_Timer_C|GetTimeLeft _timerref))
  (bind _returnvalue_2 (Math|Conversions|ToFloat(Integer) _timeleft))
  (bind _returnvalue_3 (/ _returnvalue_2 1e+02))
  (bind _returnvalue_4 (* _returnvalue_3 1.2))
  (bind _returnvalue_5 (Math|Float|Clamp(Float) _returnvalue_4 0.3))
  (if (> (Variables|/Game/Widget/WB_Timer.WB_Timer_C|GetTimeLeft (Variables|/Game/GameMode/BP_GameMode.BP_GameMode_C|GetTimerRef (Variables|Default|GetAs%20BP%20Game%20Mode))) 0)
    (Rendering|Components|Light|SetLightColor (Variables|/Script/Engine.Light|GetLightComponent (Variables|Default|GetDirectionnalLight)) (Utilities|Struct|MakeLinearColor (.r _returnvalue) _returnvalue_5 _returnvalue_5 (.a _returnvalue)) true)))

(event EventBeginPlay
  (bind _asbp_game_mode (Utilities|Casting|CastToBP_GameMode (Game|GetGameMode)))
  (Variables|Default|SetAs%20BP%20Game%20Mode _asbp_game_mode)
  (bind _asbp_third_person_character (Utilities|Casting|CastToBP_ThirdPersonCharacter (Game|GetPlayerCharacter 0)))
  (Variables|Default|SetAs%20BP%20Third%20Person%20Character _asbp_third_person_character)
  (Utilities|Time|SetTimerbyEvent (EventDispatchers|CreateEvent :!event Custom|ChangeColor) 0.25 true true))

(event Collision|EventActorBeginOverlap
  (params (OtherActor :type Actor%20Object%20Reference)))

(event EventTick
  (params (DeltaSeconds :type Float%20%28single-precision%29)))

(fn ConstructionScript)