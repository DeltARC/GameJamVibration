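; BP_Chien is a dog NPC that patrols a list of waypoint actors from BeginPlay.
; AI MoveTo drives the movement, advancing a counter on each success and resetting it past the list's end to keep looping.
; A failed move retries after a short delay.
; On actor overlap, it prints the force calculated by BPColisionForce, with no other reaction.
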(event Custom|Lane
  (bind _waypoints (Variables|Default|GetWayPoints))
  (bind _output_get (Variables|Default|SetLengthListOfDirectionPoint (Utilities|Array|Length _waypoints)))
  (AI|AIMoveTo self "0, 0, 0" (Utilities|Array|Get(acopy) _waypoints (stale _result)) 1e+02 false :!label _label
    (:OnSuccess
      (bind _result (Math|Integer|IncrementInt (Variables|Default|GetNumberOfListDirection))
        (:%20%20
          (if (>= (Variables|Default|GetNumberOfListDirection) _output_get)
            (Variables|Default|SetNumberOfListDirection -1)
            (goto _label)
            (else
              (goto _label))))))
    (:OnFail
      (Utilities|FlowControl|Delay 2.0)
      (goto _label))))

(event EventBeginPlay
  (CallFunction|Lane))

(event Collision|EventActorBeginOverlap
  (params (OtherActor :type Actor%20Object%20Reference))
  (Development|PrintString (Utilities|String|ToString(Vector2d) (Default|CalculateForce (Variables|Default|GetBP_ColisionForce)))))

(fn ConstructionScript)