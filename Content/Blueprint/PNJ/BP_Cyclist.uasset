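; Cyclist NPC that rides a looping waypoint route and knocks the player away when they overlap.
; AI MoveTo advances through the WayPoints list, moving on after a short delay if a move fails.
; It binds to GameMode's red and green light events, with stop and restart logic that toggles walk speed via a polling timer and CanStop flag.
; Overlap launches the player using BPColisionForce's computed velocity.
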(event Custom|StopCar
  (bind _returnvalue (Utilities|Time|SetTimerbyEvent (delegate Custom|Stop) 0.15 true))
  (Variables|Default|SetTimerStop _returnvalue))

(event Custom|Lane
  (bind _waypoints (Variables|Default|GetWayPoints))
  (bind _output_get (Variables|Default|SetLengthListOfDirectionPoint (Utilities|Array|Length _waypoints)))
  (AI|AIMoveTo self "0, 0, 0" (Utilities|Array|Get(acopy) _waypoints (Variables|Default|GetNumberOfListDirection)) 1e+02 false :!label _label
    (:OnSuccess
      (Math|Integer|IncrementInt (Variables|Default|GetNumberOfListDirection)
        (:%20%20
          _)))
    (:OnFail
      (Utilities|FlowControl|Delay 2.0)))
  (if (> (+ (Variables|Default|GetNumberOfListDirection) 1) _output_get)
    (Variables|Default|SetNumberOfListDirection 0)
    (goto _label)
    (else
      (goto _label))))

(event Custom|Stop
  (if (Variables|Default|GetCanStop?)
    (Variables|/Script/Engine.CharacterMovementComponent|SetMaxWalkSpeed (Variables|Character|GetCharacterMovement) 1e-05)
    (else
      (Variables|/Script/Engine.CharacterMovementComponent|SetMaxWalkSpeed (Variables|Character|GetCharacterMovement) (Variables|Default|GetMaxWalkSpeedBase)))))

(event Custom|RestartCar
  (Utilities|Time|ClearandInvalidateTimerbyHandle (Variables|Default|GetTimerStop))
  (Variables|/Script/Engine.CharacterMovementComponent|SetMaxWalkSpeed (Variables|Character|GetCharacterMovement) (Variables|Default|GetMaxWalkSpeedBase)))

(event EventBeginPlay
  (bind _asbp_third_person_character (Utilities|Casting|CastToBP_ThirdPersonCharacter (Game|Player|GetPlayerPawn 0)))
  (Variables|Default|SetAs%20BP%20Third%20Person%20Character _asbp_third_person_character)
  (CallFunction|Lane)
  (bind _asbp_game_mode (Utilities|Casting|CastToBP_GameMode (Game|GetGameMode)))
  (bind _output_get (Variables|Default|SetAs%20BP%20Game%20Mode _asbp_game_mode))
  (EventDispatchers|BindEventtoLightRed _output_get (EventDispatchers|CreateEvent :!event Custom|StopCar))
  (Variables|Default|SetMaxWalkSpeedBase (Variables|/Script/Engine.CharacterMovementComponent|GetMaxWalkSpeed (Variables|Character|GetCharacterMovement)))
  (EventDispatchers|BindEventtoLightGreen (Variables|Default|GetAs%20BP%20Game%20Mode) (EventDispatchers|CreateEvent :!event Custom|RestartCar)))

(event Collision|EventActorBeginOverlap
  (params (OtherActor :type Actor%20Object%20Reference))
  (bind _bp_colisionforce (Variables|Default|GetBP_ColisionForce))
  (if (== OtherActor (Variables|Default|GetAs%20BP%20Third%20Person%20Character))
    (Development|PrintString (Utilities|String|ToString(Vector2d) (Default|CalculateForce _bp_colisionforce)))
    (bind _lauchvelocityvector (Default|CalculateLaunchVelocity _bp_colisionforce))
    (Character|LaunchCharacter (Variables|Default|GetAs%20BP%20Third%20Person%20Character) (* _lauchvelocityvector (Variables|Default|Getvelocity)) false false)))

(fn ConstructionScript)