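; Patrolling NPC pawn that walks a looping route of waypoints and knocks the player back on overlap.
; Lane chains AI MoveTo calls through the WayPoints array, wrapping at the end and retrying two seconds after a failed move.
; Any actor overlap prints a force from BPColisionForce and launches the cached third-person player character, using its computed launch velocity scaled by Velocity.
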(event Custom|Lane
  (bind _waypoints (Variables|Default|GetWayPoints))
  (bind _output_get (Variables|Default|SetLengthListOfDirectionPoint (Utilities|Array|Length _waypoints)))
  (AI|AIMoveTo self "0, 0, 0" (Utilities|Array|Get(acopy) _waypoints (stale _result)) 1e+02 true :!label _label
    (:OnSuccess
      (bind _result (Math|Integer|IncrementInt (Variables|Default|GetNumberOfListDirection))
        (:%20%20
          _)))
    (:OnFail
      (Utilities|FlowControl|Delay 2.0)))
  (if (>= (Variables|Default|GetNumberOfListDirection) _output_get)
    (Variables|Default|SetNumberOfListDirection -1)
    (goto _label)
    (else
      (goto _label))))

(event EventBeginPlay
  (bind _asbp_third_person_character (Utilities|Casting|CastToBP_ThirdPersonCharacter (Game|Player|GetPlayerPawn 0)))
  (Variables|Default|SetAs%20BP%20Third%20Person%20Character _asbp_third_person_character)
  (CallFunction|Lane))

(event Collision|EventActorBeginOverlap
  (params (OtherActor :type Actor%20Object%20Reference))
  (bind _bp_colisionforce (Variables|Default|GetBP_ColisionForce))
  (Development|PrintString (Utilities|String|ToString(Vector2d) (Default|CalculateForce _bp_colisionforce)))
  (bind _lauchvelocityvector (Default|CalculateLaunchVelocity _bp_colisionforce))
  (Character|LaunchCharacter (Variables|Default|GetAs%20BP%20Third%20Person%20Character) (* _lauchvelocityvector (Variables|Default|Getvelocity)) false false))

(fn ConstructionScript)