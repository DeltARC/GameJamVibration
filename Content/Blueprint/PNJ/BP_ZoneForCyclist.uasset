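; BP_ZoneForCyclist is a trigger zone, apparently for cyclist NPCs, that toggles player following on a set of waypoints.
; When a BP_ThirdPersonCharacter enters the Box, it stores the character and passes it to FollowPlayer on every entry in WayPoints.
; When that character leaves, it calls ClearTimer on each entry; the follow logic itself lives in the waypoints.
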(event OnComponentBeginOverlap(Box)
  (params (OverlappedComponent :type Primitive%20Component%20Object%20Reference) (OtherActor :type Actor%20Object%20Reference) (OtherComp :type Primitive%20Component%20Object%20Reference) (OtherBodyIndex :type Integer) (bFromSweep :type Boolean) (SweepResult :type Hit%20Result%20Structure%20%28by%20ref%29))
  (bind _asbp_third_person_character (Utilities|Casting|CastToBP_ThirdPersonCharacter OtherActor))
  (Variables|Default|SetAs%20BP%20Third%20Person%20Character _asbp_third_person_character)
  (for _array_element (Variables|Default|GetWayPoints)
    (Default|FollowPlayer _array_element (Variables|Default|GetAs%20BP%20Third%20Person%20Character))))

(event OnComponentEndOverlap(Box)
  (params (OverlappedComponent :type Primitive%20Component%20Object%20Reference) (OtherActor :type Actor%20Object%20Reference) (OtherComp :type Primitive%20Component%20Object%20Reference) (OtherBodyIndex :type Integer))
  (Utilities|Casting|CastToBP_ThirdPersonCharacter OtherActor)
  (for _array_element (Variables|Default|GetWayPoints)
    (Default|ClearTimer _array_element)))

(fn ConstructionScript)