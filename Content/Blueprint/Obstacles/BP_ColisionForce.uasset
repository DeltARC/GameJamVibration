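; Scene component in the obstacles folder that works out the direction of a collision force relative to the player pawn.
; CalculateForce takes the normalized vector from the component's world location to player 0's pawn.
; It dots that vector with the pawn's forward and right vectors, returning the results as X and Y force directions.
; It only computes these values and applies no force; the event graph is empty.
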(event EventBeginPlay)

(event EventTick
  (params (DeltaSeconds :type Float%20%28single-precision%29)))

(fn CalculateForce
  (bind _returnvalue (Game|Player|GetPlayerPawn 0))
  (bind _returnvalue_2 (Transformation|GetWorldLocation))
  (bind _returnvalue_3 (Transformation|GetActorLocation _returnvalue))
  (bind _returnvalue_4 (- _returnvalue_3 _returnvalue_2))
  (bind _returnvalue_5 (Math|Vector|Normalize _returnvalue_4))
  (return (Math|Vector2D|MakeVector2D (Math|Vector|DotProduct (Math|Vector|Normalize (Transformation|GetActorForwardVector _returnvalue)) _returnvalue_5) (Math|Vector|DotProduct (Transformation|GetActorRightVector _returnvalue) _returnvalue_5))))