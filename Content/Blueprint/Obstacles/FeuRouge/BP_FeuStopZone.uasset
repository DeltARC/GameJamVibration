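; BP_FeuStopZone is a trigger zone in the traffic light (FeuRouge) obstacle set that marks where patrol pawns are allowed to stop.
; When a BP_PatrolPawn begins overlapping its Box, the zone sets that pawn's CanStop to true, and resets it to false when the overlap ends.
; It holds no light-state logic and only toggles this flag on the pawn.
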(event OnComponentBeginOverlap(Box)
  (params (OverlappedComponent :type Primitive%20Component%20Object%20Reference) (OtherActor :type Actor%20Object%20Reference) (OtherComp :type Primitive%20Component%20Object%20Reference) (OtherBodyIndex :type Integer) (bFromSweep :type Boolean) (SweepResult :type Hit%20Result%20Structure%20%28by%20ref%29))
  (bind _asbp_patrol_pawn (Utilities|Casting|CastToBP_PatrolPawn OtherActor))
  (Variables|Default|SetAs%20BP%20Patrol%20Pawn _asbp_patrol_pawn)
  (if (== _asbp_patrol_pawn OtherActor)
    (Variables|/Game/Blueprint/PNJ/BP_PatrolPawn.BP_PatrolPawn_C|SetCanStop? (Variables|Default|GetAs%20BP%20Patrol%20Pawn) true)))

(event OnComponentEndOverlap(Box)
  (params (OverlappedComponent :type Primitive%20Component%20Object%20Reference) (OtherActor :type Actor%20Object%20Reference) (OtherComp :type Primitive%20Component%20Object%20Reference) (OtherBodyIndex :type Integer))
  (bind _asbp_patrol_pawn (Utilities|Casting|CastToBP_PatrolPawn OtherActor))
  (Variables|Default|SetAs%20BP%20Patrol%20Pawn _asbp_patrol_pawn)
  (if (== _asbp_patrol_pawn OtherActor)
    (Variables|/Game/Blueprint/PNJ/BP_PatrolPawn.BP_PatrolPawn_C|SetCanStop? (Variables|Default|GetAs%20BP%20Patrol%20Pawn) false)))

(event EventBeginPlay)

(event Collision|EventActorBeginOverlap
  (params (OtherActor :type Actor%20Object%20Reference)))

(event EventTick
  (params (DeltaSeconds :type Float%20%28single-precision%29)))

(fn ConstructionScript)