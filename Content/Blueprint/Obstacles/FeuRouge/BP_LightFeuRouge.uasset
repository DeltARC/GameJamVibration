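; BP_LightFeuRouge is a traffic light obstacle actor that shows red or green through two light components, FeuRouge and FeuVert.
; On BeginPlay it binds to the light-red and light-green events on BP_GameMode, so the game mode drives the switching.
; RedLight and GreenLight swap the two intensities between bright and near zero, with PlayerInverse reversing the colour shown.
; The non-inverted branches also print leftover debug strings.
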(event Custom|GreenLight
  (if (Variables|Default|GetPlayerInverse)
    (Rendering|Components|Light|SetIntensity (Variables|Default|GetFeuRouge) 65.0)
    (Rendering|Components|Light|SetIntensity (Variables|Default|GetFeuVert) 0.001)
    (else
      (Rendering|Components|Light|SetIntensity (Variables|Default|GetFeuRouge) 0.001)
      (Rendering|Components|Light|SetIntensity (Variables|Default|GetFeuVert) 65.0)
      (Development|PrintString "55"))))

(event Custom|RedLight
  (if (Variables|Default|GetPlayerInverse)
    (Rendering|Components|Light|SetIntensity (Variables|Default|GetFeuRouge) 0.001)
    (Rendering|Components|Light|SetIntensity (Variables|Default|GetFeuVert) 65.0)
    (else
      (Rendering|Components|Light|SetIntensity (Variables|Default|GetFeuRouge) 65.0)
      (Rendering|Components|Light|SetIntensity (Variables|Default|GetFeuVert) 0.001)
      (Development|PrintString "Hello"))))

(event EventBeginPlay
  (bind _asbp_game_mode (Utilities|Casting|CastToBP_GameMode (Game|GetGameMode)))
  (bind _output_get (Variables|Default|SetAs%20BP%20Game%20Mode _asbp_game_mode))
  (EventDispatchers|BindEventtoLightRed _output_get (EventDispatchers|CreateEvent :!event Custom|RedLight))
  (EventDispatchers|BindEventtoLightGreen (Variables|Default|GetAs%20BP%20Game%20Mode) (EventDispatchers|CreateEvent :!event Custom|GreenLight)))

(event Collision|EventActorBeginOverlap
  (params (OtherActor :type Actor%20Object%20Reference)))

(event EventTick
  (params (DeltaSeconds :type Float%20%28single-precision%29)))

(fn ConstructionScript)