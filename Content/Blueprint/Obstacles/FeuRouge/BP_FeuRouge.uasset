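; BP_FeuRouge is a traffic light obstacle that signals red and green phases to BP_GameMode.
; A looping timer started on BeginPlay switches the referenced NavMesh actor to its activated scale and calls the game mode's red light.
; After a Delay equal to the timer interval, it restores the base scale and calls green, so the reset coincides with the next timer tick.
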(event Custom|FeuRougeEvent
  (Transformation|SetActorScale3D (Variables|Default|GetNavMesh) (Variables|Default|GetScaleActivated))
  (Default|CallLightRed (Variables|Default|GetAs%20BP%20Game%20Mode))
  (Utilities|FlowControl|Delay 8.0)
  (Transformation|SetActorScale3D (Variables|Default|GetNavMesh) (Variables|Default|GetScaleBase))
  (Default|CallLightGreen (Variables|Default|GetAs%20BP%20Game%20Mode)))

(event EventBeginPlay
  (bind _asbp_game_mode (Utilities|Casting|CastToBP_GameMode (Game|GetGameMode)))
  (Variables|Default|SetAs%20BP%20Game%20Mode _asbp_game_mode)
  (Utilities|Time|SetTimerbyEvent (delegate Custom|FeuRougeEvent) 8.0 true))

(event Collision|EventActorBeginOverlap
  (params (OtherActor :type Actor%20Object%20Reference)))

(event EventTick
  (params (DeltaSeconds :type Float%20%28single-precision%29)))

(fn ConstructionScript)